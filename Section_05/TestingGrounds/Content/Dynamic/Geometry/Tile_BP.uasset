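; Tile actor for infinite terrain that gates the player with a barrier wall and removes itself when the player reaches its destroy volume.
; The barrier starts solid and red, turning passable and green while the player overlaps LevelBounds.
; Leaving those bounds relocks it and asks InfiniteTerrainGameMode to spawn the next tile.
; An Arrow component supplies the attach transform, and overlap events are filtered to the player character.
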(event OnComponentEndOverlap(LevelBounds)
  (params (OverlappedComponent :type Primitive%20Component%20Object%20Reference) (OtherActor :type Actor%20Object%20Reference) (OtherComp :type Primitive%20Component%20Object%20Reference) (OtherBodyIndex :type Integer))
  (Utilities|IsPlayerActor OtherActor)
  (CallFunction|Lock)
  (bind _asinfinite_terrain_game_mode (Utilities|Casting|CastToInfiniteTerrainGameMode (Game|GetGameMode)))
  (Default|SpawnNextTile _asinfinite_terrain_game_mode))

(event OnComponentBeginOverlap(LevelBounds)
  (params (OverlappedComponent :type Primitive%20Component%20Object%20Reference) (OtherActor :type Actor%20Object%20Reference) (OtherComp :type Primitive%20Component%20Object%20Reference) (OtherBodyIndex :type Integer) (bFromSweep :type Boolean) (SweepResult :type Hit%20Result%20Structure%20%28by%20ref%29))
  (Utilities|IsPlayerActor OtherActor)
  (CallFunction|Unlock))

(event OnComponentBeginOverlap(LevelDestroyVolume)
  (params (OverlappedComponent :type Primitive%20Component%20Object%20Reference) (OtherActor :type Actor%20Object%20Reference) (OtherComp :type Primitive%20Component%20Object%20Reference) (OtherBodyIndex :type Integer) (bFromSweep :type Boolean) (SweepResult :type Hit%20Result%20Structure%20%28by%20ref%29))
  (Utilities|IsPlayerActor OtherActor)
  (Actor|DestroyActor))

(event EventBeginPlay
  (CallFunction|Lock))

(fn ConstructionScript)

(fn GetAttachLocation
  (return (Transformation|GetWorldTransform (Variables|Default|GetArrow))))

(fn Unlock
  (bind _barrier_wall (Variables|Default|GetBarrier%20Wall))
  (Collision|SetCollisionEnabled _barrier_wall "NoCollision")
  (Rendering|Material|SetMaterial _barrier_wall 0 "/Game/Static/Geometry/Materials/MaterialInstances/Barrier_Green.Barrier_Green"))

(fn Lock
  (bind _barrier_wall (Variables|Default|GetBarrier%20Wall))
  (Collision|SetCollisionEnabled _barrier_wall "QueryAndPhysics")
  (Rendering|Material|SetMaterial _barrier_wall 0 "/Game/Static/Geometry/Materials/MaterialInstances/Barrier_Red.Barrier_Red"))
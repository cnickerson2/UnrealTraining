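; Terrain tile for the infinite terrain game mode that scatters props and gates the player with a barrier wall.
; On BeginPlay it passes rocks, containers and smaller props to PlaceActors with count, scale and clearance-radius settings, then locks the barrier.
; The player entering LevelBounds unlocks it (green, no collision), and leaving relocks it (red, solid).
; Player overlap with LevelDestroyVolume destroys the tile and requests the next; an Arrow supplies the attach transform.
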(event OnComponentEndOverlap(LevelBounds)
  (params (OverlappedComponent :type Primitive%20Component%20Object%20Reference) (OtherActor :type Actor%20Object%20Reference) (OtherComp :type Primitive%20Component%20Object%20Reference) (OtherBodyIndex :type Integer))
  (Utilities|IsPlayerActor OtherActor)
  (CallFunction|Lock))

(event OnComponentBeginOverlap(LevelBounds)
  (params (OverlappedComponent :type Primitive%20Component%20Object%20Reference) (OtherActor :type Actor%20Object%20Reference) (OtherComp :type Primitive%20Component%20Object%20Reference) (OtherBodyIndex :type Integer) (bFromSweep :type Boolean) (SweepResult :type Hit%20Result%20Structure%20%28by%20ref%29))
  (Utilities|IsPlayerActor OtherActor)
  (CallFunction|Unlock))

(event OnComponentBeginOverlap(LevelDestroyVolume)
  (params (OverlappedComponent :type Primitive%20Component%20Object%20Reference) (OtherActor :type Actor%20Object%20Reference) (OtherComp :type Primitive%20Component%20Object%20Reference) (OtherBodyIndex :type Integer) (bFromSweep :type Boolean) (SweepResult :type Hit%20Result%20Structure%20%28by%20ref%29))
  (Utilities|IsPlayerActor OtherActor)
  (Actor|DestroyActor)
  (bind _asgame_mode_infinite_terrain (Utilities|Casting|CastToGameMode_InfiniteTerrain (Game|GetGameMode)))
  (Default|SpawnNextTile _asgame_mode_infinite_terrain))

(event EventBeginPlay
  (CallFunction|SpawnAllProps)
  (CallFunction|Lock))

(fn ConstructionScript)

(fn GetAttachLocation
  (return (Transformation|GetWorldTransform (Variables|Default|GetArrow))))

(fn Unlock
  (bind _barrier_wall (Variables|Default|GetBarrier%20Wall))
  (Collision|SetCollisionEnabled _barrier_wall "NoCollision")
  (Rendering|Material|SetMaterial _barrier_wall 0 "/Game/TestingGrounds/Static/Geometry/Materials/MaterialInstances/MI_Barrier_Green.MI_Barrier_Green"))

(fn Lock
  (bind _barrier_wall (Variables|Default|GetBarrier%20Wall))
  (Collision|SetCollisionEnabled _barrier_wall "QueryAndPhysics")
  (Rendering|Material|SetMaterial _barrier_wall 0 "/Game/TestingGrounds/Static/Geometry/Materials/MaterialInstances/MI_Barrier_Red.MI_Barrier_Red"))

(fn SpawnAllProps
  (bind _maxrockscalingsize (LocalVariables|GetMaxRockScalingSize))
  (CallFunction|SpawnProp "/Game/TestingGrounds/Dynamic/Geometry/Props/BP_Rock_01.BP_Rock_01_C" 0 4 1.0 _maxrockscalingsize 3e+02)
  (CallFunction|SpawnProp "/Game/TestingGrounds/Dynamic/Geometry/Props/BP_Rock_02.BP_Rock_02_C" 0 4 1.0 _maxrockscalingsize 275.0)
  (CallFunction|SpawnProp "/Game/TestingGrounds/Dynamic/Geometry/Props/BP_Rock_03.BP_Rock_03_C" 0 4 1.0 _maxrockscalingsize 2.5e+02)
  (CallFunction|SpawnProp "/Game/TestingGrounds/Dynamic/Geometry/Props/BP_Container.BP_Container_C" 1 3 1.0 1.0 4e+02)
  (CallFunction|SpawnProp "/Game/TestingGrounds/Dynamic/Geometry/Props/BP_SandBags.BP_SandBags_C" 0 2 1.0 1.0 1.5e+02)
  (CallFunction|SpawnProp "/Game/TestingGrounds/Dynamic/Geometry/Props/BP_Box.BP_Box_C" 2 4 1.0 1.0 1e+02)
  (CallFunction|SpawnProp "/Game/TestingGrounds/Dynamic/Geometry/Props/BP_Canister.BP_Canister_C" 1 7 1.0 1.0 5e+01))

(fn SpawnProp
  (params (Prop%20to%20Spawn :type Actor%20Class%20Reference) (Min%20Spawn :type Integer) (Max%20Spawn :type Integer) (Min%20Possible%20Scaling :type Float%20%28single-precision%29) (Max%20Possible%20Scaling :type Float%20%28single-precision%29) (Acceptable%20Radius :type Float%20%28single-precision%29))
  (Class|Tile|PlaceActors Prop%20to%20Spawn (Utilities|Struct|MakeSpawningAttributes Min%20Spawn Max%20Spawn Min%20Possible%20Scaling Max%20Possible%20Scaling Acceptable%20Radius)))
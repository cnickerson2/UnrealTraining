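; AI controller for guard NPCs that runs the GuardBehaviour tree on PatrolData and drives combat on the controlled Character_BP.
; Perception stores sensed actors lacking the "Enemy" tag as the blackboard target; losing sight clears it and saves that target's location as last seen.
; Tick sets the pawn's Aiming and Shooting flags whenever a focus actor is valid.
; A debug helper logs perceived senses.
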(event OnTargetPerceptionUpdated(AIPerception)
  (params (Actor :type Actor%20Object%20Reference) (Stimulus :type AI%20Stimulus%20Structure))
  (bind _blackboardcomp (Variables|Default|GetBlackboardComp))
  (bind _enemykey (Variables|Default|GetEnemyKey))
  (if (not (Actor|ActorHasTag Actor "Enemy"))
    (if (.bSuccessfullySensed (Utilities|Struct|BreakAIStimulus Stimulus))
      (AI|Components|Blackboard|SetValueasObject _blackboardcomp _enemykey Actor)
      (else
        (bind _asactor (Utilities|Casting|CastToActor (AI|Components|Blackboard|GetValueasObject _blackboardcomp _enemykey)))
        (AI|Components|Blackboard|ClearValue _blackboardcomp _enemykey)
        (AI|Components|Blackboard|SetValueasVector _blackboardcomp (Variables|Default|GetLastSeenLocationKey) (Transformation|GetActorLocation _asactor))))))

(event EventBeginPlay
  (bind _blackboardcomponent (Class|AIController|UseBlackboard "/Game/Dynamic/Character/AI/PatrolData.PatrolData"))
  (AI|RunBehaviorTree "/Game/Dynamic/Character/AI/GuardBehaviour.GuardBehaviour")
  (Variables|Default|SetBlackboardComp _blackboardcomponent))

(event EventTick
  (params (DeltaSeconds :type Float%20%28single-precision%29))
  (bind _returnvalue (Class|AIController|GetFocusActor))
  (bind _returnvalue_2 (Utilities|IsValid _returnvalue))
  (bind _ascharacter_bp (Utilities|Casting|CastToCharacter_BP (Pawn|GetControlledPawn)))
  (Variables|/Game/Dynamic/Character/Behaviour/Character_BP.Character_BP_C|SetAiming _ascharacter_bp _returnvalue_2)
  (Variables|/Game/Dynamic/Character/Behaviour/Character_BP.Character_BP_C|SetShooting _ascharacter_bp _returnvalue_2))

(fn ConstructionScript)

(fn PrintOutPerception
  (params (Object :type Object%20Object%20Reference) (Stimulus :type AI%20Stimulus%20Structure%20%28by%20ref%29))
  (bind _returnvalue (Class|AIPerceptionSystem|GetSenseClassforStimulus Stimulus))
  (Development|PrintString (Utilities|String|Append (Utilities|GetDisplayName (Pawn|GetControlledPawn)) " " (Utilities|GetClassDisplayName _returnvalue) " " (Utilities|GetDisplayName Object)) false))